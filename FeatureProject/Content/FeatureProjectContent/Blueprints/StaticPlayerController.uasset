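; Player controller that shows the mouse cursor and sends every pathfinding agent in the level toward a clicked floor point.
; On left click it traces under the cursor, draws a debug line, and continues only if the hit actor is tagged "floor".
; It then scans all actors for JPS, A* and JPS+ agent components, cancelling each one's current path and requesting a new path to the hit location.
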(event EventBeginPlay
  (Variables|Default|SetbShowMouseCursor true))

(event Input|MouseEvents|LeftMouseButton
  (params (Key :type Key%20Structure :default "AnyKey"))
  (bind _hitresult (Game|Player|GetHitResultUnderCursorbyChannel "TraceTypeQuery1" true))
  (bind (_bblockinghit _binitialoverlap _time _location _impactpoint _normal _impactnormal _physmat _hitactor _hitcomponent _hitbonename _hititem _tracestart) (Collision|BreakHitResult _hitresult))
  (:Pressed
    (Rendering|Debug|DrawDebugLine (- _tracestart "0, 0,200.000000") _location (Utilities|Struct|MakeLinearColor 0.0 1.0 0.0 0.0) 2.0 1.0)
    (Utilities|IsValid _hitactor
      (:Is%20Valid
        (if (Actor|ActorHasTag _hitactor "floor")
          (bind _outactors (Actor|GetAllActorsOfClass "/Script/Engine.Actor"))
          (for _array_element _outactors
            (Utilities|FlowControl|Sequence
              (:then_0
                (if (> (Utilities|Array|Length (Actor|GetComponentsByClass _array_element "/Script/FeatureProject.JPSAgentComponent")) 0)
                  (Utilities|IsValid (Utilities|Array|Get(acopy) (Actor|GetComponentsByClass _array_element "/Script/FeatureProject.JPSAgentComponent"))
                    (:Is%20Valid
                      (Class|JPSAgentComponent|CancelCurrentPath (Utilities|Array|Get(acopy) (Actor|GetComponentsByClass _array_element "/Script/FeatureProject.JPSAgentComponent")))
                      (Class|JPSAgentComponent|CalculatePointsandRequestPath (Utilities|Array|Get(acopy) (Actor|GetComponentsByClass _array_element "/Script/FeatureProject.JPSAgentComponent")) _location)))))
              (:then_1
                (if (> (Utilities|Array|Length (Actor|GetComponentsByClass _array_element "/Script/FeatureProject.AStarAgentComponent")) 0)
                  (Utilities|IsValid (Utilities|Array|Get(acopy) (Actor|GetComponentsByClass _array_element "/Script/FeatureProject.AStarAgentComponent"))
                    (:Is%20Valid
                      (Class|AStarAgentComponent|CancelCurrentPath (Utilities|Array|Get(acopy) (Actor|GetComponentsByClass _array_element "/Script/FeatureProject.AStarAgentComponent")))
                      (Class|AStarAgentComponent|CalculatePointsandRequestPath (Utilities|Array|Get(acopy) (Actor|GetComponentsByClass _array_element "/Script/FeatureProject.AStarAgentComponent")) _location)))))
              (:then_2
                (if (> (Utilities|Array|Length (Actor|GetComponentsByClass _array_element "/Script/FeatureProject.JPSPlusAgentComponent")) 0)
                  (Utilities|IsValid (Utilities|Array|Get(acopy) (Actor|GetComponentsByClass _array_element "/Script/FeatureProject.JPSPlusAgentComponent"))
                    (:Is%20Valid
                      (Class|JPSPlusAgentComponent|CancelCurrentPath (Utilities|Array|Get(acopy) (Actor|GetComponentsByClass _array_element "/Script/FeatureProject.JPSPlusAgentComponent")))
                      (Class|JPSPlusAgentComponent|CalculatePointsandRequestPath (Utilities|Array|Get(acopy) (Actor|GetComponentsByClass _array_element "/Script/FeatureProject.JPSPlusAgentComponent")) _location))))))))))))

(fn ConstructionScript)